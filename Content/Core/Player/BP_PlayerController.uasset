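; Player controller for RTS-style play, handling camera control, pause toggling, and unit selection and movement.
; Enhanced Input forwards camera actions to BP_CameraPawn and pause to BP_GameState, with full tick during pause for camera movement.
; Drag selection records mouse coordinates for external use and suspends edge scrolling.
; SetSelectedUnits stores actors' BP_RadioControlUnit components, optionally keeping prior selection, and destination clicks move them to the cursor trace location.
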(event `self.ReceiveBeginPlay`
  (bind _returnvalue (subsystem `EnhancedInputLocalPlayerSubsystem`))
  (set `self.bShouldPerformFullTickWhenPaused` true) ; Can move camera when paused
  (bind _asbp_camera_pawn (cast `/Game/Core/Player/BP_CameraPawn` (`GameplayStatics.GetPlayerPawn` 0)))
  (set `self.CameraPawnRef` _asbp_camera_pawn)
  (bind _asbp_game_state (cast `/Game/Core/Settings/BP_GameState` (`GameplayStatics.GetGameState`)))
  (set `self.GameStateRef` _asbp_game_state)
  ;[1 1 1] Initialize inputs
  (set `self.bShowMouseCursor` true) ; Make cursor visible
  (`/Engine/EditorBlueprintResources/StandardMacros.IsValid` _returnvalue
    (:`Is Valid`
      (`EnhancedInputSubsystemInterface.AddMappingContext` _returnvalue "/Game/Core/Inputs/IMC_PC.IMC_PC" 0 (struct)))))

(event `EnhancedInput|/Game/Core/Inputs/Actions/Camera/IA_MoveCamera`
  (params (ActionValue :type "Vector2D Structure") (ElapsedSeconds :type "Float (double-precision)") (TriggeredSeconds :type "Float (double-precision)") (InputAction :type "InputAction Object Reference" :default "/Game/Core/Inputs/Actions/Camera/IA_MoveCamera.IA_MoveCamera"))
  ;[1 1 1] Camera Controls
  (:`Triggered`
    (`/Game/Core/Player/BP_CameraPawn.MoveCamera` (`self.CameraPawnRef`) ActionValue_X ActionValue_Y)))

(event `EnhancedInput|/Game/Core/Inputs/Actions/IA_PauseGame`
  (params (ActionValue :type Boolean) (ElapsedSeconds :type "Float (double-precision)") (TriggeredSeconds :type "Float (double-precision)") (InputAction :type "InputAction Object Reference" :default "/Game/Core/Inputs/Actions/IA_PauseGame.IA_PauseGame"))
  (:`Started`
    (`/Game/Core/Settings/BP_GameState.SwitchPause` (`self.GameStateRef`))))

(event `EnhancedInput|/Game/Core/Inputs/Actions/Camera/IA_ZoomCamera`
  (params (ActionValue :type "Float (double-precision)") (ElapsedSeconds :type "Float (double-precision)") (TriggeredSeconds :type "Float (double-precision)") (InputAction :type "InputAction Object Reference" :default "/Game/Core/Inputs/Actions/Camera/IA_ZoomCamera.IA_ZoomCamera"))
  ;[1 1 1] Camera Controls
  (:`Triggered`
    (`/Game/Core/Player/BP_CameraPawn.ZoomCamera` (`self.CameraPawnRef`) ActionValue)))

(event `EnhancedInput|/Game/Core/Inputs/Actions/IA_SetDestination`
  (params (ActionValue :type Boolean) (ElapsedSeconds :type "Float (double-precision)") (TriggeredSeconds :type "Float (double-precision)") (InputAction :type "InputAction Object Reference" :default "/Game/Core/Inputs/Actions/IA_SetDestination.IA_SetDestination"))
  (:`Started`
    (for _array_element (`self.SelectedUnits`)
      (`/Game/Blueprints/Units/BP_RadioControlUnit.MoveToLocation` _array_element (`.Location` (`self.GetLocaltionUnderCursor`))))))

(event `EnhancedInput|/Game/Core/Inputs/Actions/Camera/IA_SpeedCamera`
  (params (ActionValue :type Boolean) (ElapsedSeconds :type "Float (double-precision)") (TriggeredSeconds :type "Float (double-precision)") (InputAction :type "InputAction Object Reference" :default "/Game/Core/Inputs/Actions/Camera/IA_SpeedCamera.IA_SpeedCamera"))
  ;[1 1 1] Camera Controls
  (:`Triggered`
    (`/Game/Core/Player/BP_CameraPawn.SetSpeedUp` (`self.CameraPawnRef`) ActionValue)))

(event `EnhancedInput|/Game/Core/Inputs/Actions/Selection/IA_SetSelectionZone`
  (params (ActionValue :type Boolean) (ElapsedSeconds :type "Float (double-precision)") (TriggeredSeconds :type "Float (double-precision)") (InputAction :type "InputAction Object Reference" :default "/Game/Core/Inputs/Actions/Selection/IA_SetSelectionZone.IA_SetSelectionZone"))
  (bind (_locationx _locationy) (`self.GetMousePosition`))
  (bind _returnvalue (`KismetMathLibrary.MakeVector2D` _locationx _locationy))
  ;[1 1 1] Select units
  (:`Triggered`
    (set `self.CurrentMousePosition` _returnvalue))
  (:`Started`
    (set `self.bIsDrawing` true)
    (`/Game/Core/Player/BP_CameraPawn.SetDisableEdgeScroll` (`self.CameraPawnRef`) true)
    (set `self.FirstMousePosition` _returnvalue)
    (set `self.CurrentMousePosition` _returnvalue))
  (:`Canceled`
    (set `self.bIsDrawing` false :!label _label)
    (`/Game/Core/Player/BP_CameraPawn.SetDisableEdgeScroll` (`self.CameraPawnRef`) false))
  (:`Completed`
    (goto _label)))

(event `EnhancedInput|/Game/Core/Inputs/Actions/Camera/IA_PanCamera`
  (params (ActionValue :type Boolean) (ElapsedSeconds :type "Float (double-precision)") (TriggeredSeconds :type "Float (double-precision)") (InputAction :type "InputAction Object Reference" :default "/Game/Core/Inputs/Actions/Camera/IA_PanCamera.IA_PanCamera"))
  (bind _camerapawnref (`self.CameraPawnRef`))
  ;[1 1 1] Camera Controls
  (:`Triggered`
    (`/Game/Core/Player/BP_CameraPawn.PanCamera` (`self.CameraPawnRef`) (/ (`KismetMathLibrary.MakeVector2D` (`self.GetInputAxisKeyValue`) (`self.GetInputAxisKeyValue`)) (`WidgetLayoutLibrary.GetViewportSize`))))
  (:`Started`
    (`/Game/Core/Player/BP_CameraPawn.SetDisableEdgeScroll` _camerapawnref true))
  (:`Canceled`
    (`/Game/Core/Player/BP_CameraPawn.SetDisableEdgeScroll` _camerapawnref false :!label _label_2))
  (:`Completed`
    (goto _label_2)))

(event `EnhancedInput|/Game/Core/Inputs/Actions/Selection/IA_KeepSelection`
  (params (ActionValue :type Boolean) (ElapsedSeconds :type "Float (double-precision)") (TriggeredSeconds :type "Float (double-precision)") (InputAction :type "InputAction Object Reference" :default "/Game/Core/Inputs/Actions/Selection/IA_KeepSelection.IA_KeepSelection"))
  ;[1 1 1] Select units
  (:`Triggered`
    (set `self.bKeepSelection` ActionValue)))

(event `InputVectorAxis|Mouse2D`
  (params (AxisValue :type "Vector Structure"))
  (bind (_locationx _locationy) (`self.GetMousePosition`))
  ;[1 1 1] Camera Controls
  (`/Game/Core/Player/BP_CameraPawn.EdgeScrollCamera` (`self.CameraPawnRef`) (/ (`KismetMathLibrary.MakeVector2D` _locationx _locationy) (`WidgetLayoutLibrary.GetViewportSize`))))

(event `/Game/Core/Interfaces/BPI_PlayerInputValues.SetSelectedUnits`
  (params (SelectedUnits :type "Array of Actor Object Reference (by ref)"))
  (if (not (`self.bKeepSelection`))
    (`self.ClearSelection`))
  (for _array_element SelectedUnits
    (for _array_element_2 (`self.K2_GetComponentsByClass` _array_element "/Game/Blueprints/Units/BP_RadioControlUnit.BP_RadioControlUnit_C")
      (`KismetArrayLibrary.Array_AddUnique` (`self.SelectedUnits`) _array_element_2)
      (`/Game/Blueprints/Units/BP_RadioControlUnit.Selected` _array_element_2)
      (break))))

(event `ClearSelection`
  (for _array_element (`self.SelectedUnits`)
    (`/Game/Blueprints/Units/BP_RadioControlUnit.Unselected` _array_element))
  (`KismetArrayLibrary.Array_Clear` (`self.SelectedUnits`)))

(fn `GetLocaltionUnderCursor`
  (returns (bBlockingHit :type Boolean) (Location :type "Vector Structure"))
  (bind (_bblockinghit _binitialoverlap _time _distance _location) (`GameplayStatics.BreakHitResult` (`self.GetHitResultUnderCursorByChannel` "TraceTypeQuery3")))
  (return _bblockinghit _location))

(fn `GetSelectedUnits`
  (returns (SelectedUnits :type "Array of /Game/Blueprints/Units/BP_RadioControlUnit Object Reference"))
  (return (`self.SelectedUnits`)))

(fn `MouseCoordinates`
  (returns (FirstMouseLocation :type "Vector2D Structure") (CurrentMouseLocation :type "Vector2D Structure") (bIsDrawing :type Boolean))
  (return (`self.FirstMousePosition`) (`self.CurrentMousePosition`) (`self.bIsDrawing`)))

(fn `UserConstructionScript`)