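; BP_CameraPawn is a player camera pawn with planar movement, spring-arm zoom, rotation and screen-edge scrolling, gated by a control flag.
; Movement uses swept, frame-rate-scaled local offsets with a speed-up multiplier.
; Zoom maps a normalized value through a curve to arm length, and the pawn destroys itself without that curve.
; Rotation splits actor yaw from clamped arm pitch, and active edge scrolling suspends both movement and rotation.
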(event `self.ReceiveBeginPlay`
  (bind _springarmlengthcurve (`self.SpringArmLengthCurve`)
    (:`then`
      (set `SpringArmComponent.TargetArmLength` (`CurveFloat.GetFloatValue` _springarmlengthcurve (`self.ZoomValue`)) (`self.SpringArm`)))
    (:`else`
      (`self.K2_DestroyActor`))))

(event `MoveCamera`
  (params (`X axis` :type "Float (double-precision)") (`Y axis` :type "Float (double-precision)"))
  (bind _returnvalue (`KismetMathLibrary.MakeVector` `X axis` `Y axis`))
  (bind _returnvalue_2 (`KismetMathLibrary.VSize` _returnvalue))
  ;[1 1 1] Move camera
  (if (`self.bControlCamera`)
    (if (`self.bMoveCamera`)
      (`self.K2_AddActorLocalOffset` (* _returnvalue (`KismetMathLibrary.SelectFloat` (/ 1.0 _returnvalue_2) 1.0 (> _returnvalue_2 1.0)) (`self.MoveSpeed`) (`self.SpeedMultiplier`) (`GameplayStatics.GetWorldDeltaSeconds`)) true))))

(event `ZoomCamera`
  (params (Axis :type "Float (double-precision)"))
  ;[1 1 1] Zoom camera
  (if (`self.bControlCamera`)
    (set `self.ZoomValue` (`KismetMathLibrary.FClamp` (+ (`self.ZoomValue`) (* Axis (`self.ZoomSpeed`)))))
    (set `SpringArmComponent.TargetArmLength` (`CurveFloat.GetFloatValue` (`self.SpringArmLengthCurve`) (`self.ZoomValue`)) (`self.SpringArm`))))

(event `PanCamera`
  (params (Axes :type "Vector2D Structure"))
  (bind (_returnvalue_x _returnvalue_y) (`KismetMathLibrary.BreakVector2D` (* Axes (`self.PanSensitivity`))))
  ;[1 1 1] Pan camera
  (if (`self.bControlCamera`)
    (`self.RotateCamera` _returnvalue_x _returnvalue_y)))

(event `EdgeScrollCamera`
  (params (MousePosition :type "Vector2D Structure"))
  ;[1 1 1] Edge scroll
  (if (`self.bControlCamera`)
    (`self.EdgeScroll` MousePosition)))

(fn `AddPitch`
  (params (DeltaPitch :type "Float (double-precision)"))
  (bind (_relativerotation_roll _relativerotation_pitch) (`KismetMathLibrary.BreakRotator` (`SceneComponent.RelativeRotation` (`self.SpringArm`))))
  (`SceneComponent.K2_SetRelativeRotation` (`self.SpringArm`) (`KismetMathLibrary.MakeRotator` 0.0 (`KismetMathLibrary.FClamp` (+ _relativerotation_pitch DeltaPitch) (`self.MinPitch`) (`self.MaxPitch`))) false false)
  (return))

(fn `AddYaw`
  (params (DeltaYaw :type "Float (double-precision)"))
  (bind (_returnvalue_roll _returnvalue_pitch _returnvalue_yaw) (`KismetMathLibrary.BreakRotator` (`self.K2_GetActorRotation`)))
  (`self.K2_SetActorRotation` (`KismetMathLibrary.MakeRotator` 0.0 0.0 (+ _returnvalue_yaw DeltaYaw)))
  (return))

(fn `EdgeScroll`
  (params (MousePosition :type "Vector2D Structure"))
  (locals (MoveXLocal :type "Float (double-precision)") (MoveYLocal :type "Float (double-precision)") (MouseXLocal :type "Float (double-precision)" :default 0.0) (MouseYLocal :type "Float (double-precision)" :default 0.0) (bDoScroll :type Boolean))
  (bind _bdoscroll (`local.bDoScroll`))
  (if (not (`self.bDisableEdgeScroll`))
    ;[1 1 1] Init mouse position local variables
    (set `local.MouseXLocal` MousePosition_X)
    (set `local.MouseYLocal` MousePosition_Y)
    (`|ExecutionSequence`
      (:`then_0`
        ;[1 1 1] Check movements along X axis (mouse position Y)
        (if (< (`local.MouseYLocal`) (`self.EdgeScrollBorders`))
          (set `local.MoveXLocal` 1.0)
          (set `local.bDoScroll` true :!label _label)
          (elif (> (`local.MouseYLocal`) (- 1.0 (`self.EdgeScrollBorders`)))
            (set `local.MoveXLocal` -1.0)
            (goto _label))))
      (:`then_1`
        ;[1 1 1] Check movements along Y axis (mouse position X)
        (if (< (`local.MouseXLocal`) (`self.EdgeScrollBorders`))
          (set `local.MoveYLocal` -1.0)
          (set `local.bDoScroll` true :!label _label_2)
          (elif (> (`local.MouseXLocal`) (- 1.0 (`self.EdgeScrollBorders`)))
            (set `local.MoveYLocal` 1.0)
            (goto _label_2))))
      (:`then_2`
        ;[1 1 1] Do edge scroll if have movements
        (`self.SetCameraMove` (not _bdoscroll))
        (set `self.bIsEdgeScrolling` _bdoscroll)
        (if _bdoscroll
          (`self.K2_AddActorLocalOffset` (* (`KismetMathLibrary.MakeVector` (`local.MoveXLocal`) (`local.MoveYLocal`)) (`self.EdgeScrollSpeed`) (`self.SpeedMultiplier`) (`GameplayStatics.GetWorldDeltaSeconds`)) true))))))

(fn `RotateCamera`
  (params (DeltaYaw :type "Float (double-precision)") (DeltaPitch :type "Float (double-precision)"))
  (if (`self.bMoveCamera`)
    (`self.AddYaw` DeltaYaw)
    (`self.AddPitch` DeltaPitch))
  (return))

(fn `SetCameraMove`
  (params (bMoveCamera :type Boolean))
  (set `self.bMoveCamera` bMoveCamera)
  (return))

(fn `SetControlCamera`
  (params (bControlCamera :type Boolean))
  (set `self.bControlCamera` bControlCamera)
  (return))

(fn `SetDisableEdgeScroll`
  (params (bDisableEdgeScroll :type Boolean))
  (if (not (`self.bIsEdgeScrolling`))
    (set `self.bDisableEdgeScroll` bDisableEdgeScroll))
  (return))

(fn `SetSpeedUp`
  (params (SpeedUp :type Boolean))
  (if SpeedUp
    (set `self.SpeedMultiplier` 2.0)
    (else
      (set `self.SpeedMultiplier` 1.0)))
  (return))

(fn `UserConstructionScript`)