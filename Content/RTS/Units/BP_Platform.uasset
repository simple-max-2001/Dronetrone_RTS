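; BP_Platform is an RTS unit with health and entity components that can optionally take looping timed damage from startup, apparently for death testing.
; On death it spawns an explosion and attached, time-dilated smoke, then destroys the entity after a short delay.
; Entity destruction also removes the smoke actor, and health changes print debug text showing health and alive state.
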(event `self.ReceiveBeginPlay`
  (if (`self.bDie`)
    (`KismetSystemLibrary.K2_SetTimerDelegate` (`|CreateDelegate` :!event `DieOnStartup`) 1.0 true)))

(event `DieOnStartup`
  (`HealthComponent.TakeDamage` (`self.HealthComponent`) (make `DamageData` 7.0 10.0 5.0)))

(event `self.EntityComponent.OnDieEntity`
  ;[1 1 1] On Death
  (`self.DeathFX`)
  (`KismetSystemLibrary.K2_SetTimerDelegate` (delegate `DestroyEvent`) 3.0))

(event `DestroyEvent`
  ;[1 1 1] On Death
  (`EntityComponent.DestroyEntity` (`self.EntityComponent`)))

(event `self.EntityComponent.OnDestroyEntity`
  ;[1 1 1] On Destroy
  (bind _smokeactorref (`self.SmokeActorRef`)
    (:`then`
      (`self.K2_DestroyActor` _smokeactorref))
    (:`else`)))

(event `self.HealthComponent.OnHealthChanged`
  (bind _healthcomponent (`self.HealthComponent`))
  (`KismetSystemLibrary.PrintText` (`|FormatText` "Health: {hp} ({hp_p}%) Alive: {alive}" (`HealthComponent.GetHealth` _healthcomponent) (* (`HealthComponent.GetHealthPercentage` _healthcomponent) 100.0) (`EntityComponent.IsAlive` (`self.EntityComponent`)))))

(fn `DeathFX`
  (bind (_returnvalue_location _returnvalue_rotation _returnvalue_scale) (`KismetMathLibrary.BreakTransform` (`self.GetTransform`)))
  (`|ExecutionSequence`
    (:`then_0`
      ;[1 1 1] Add explosion
      (`|SpawnActorFromClass` "/Game/RTS/FX/BP_Explosion.BP_Explosion_C" (`KismetMathLibrary.MakeTransform` (+ _returnvalue_location (0.0 0.0 100.0)) _returnvalue_rotation _returnvalue_scale) "AlwaysSpawn" "MultiplyWithRoot" null null))
    (:`then_1`
      ;[1 1 1] Add smoke
      (bind _returnvalue (`|SpawnActorFromClass` "/Game/RTS/FX/BP_Smoke.BP_Smoke_C" (`self.GetTransform`) "AlwaysSpawn" "MultiplyWithRoot" self null))
      (`self.K2_AttachToActor` _returnvalue self "None" "SnapToTarget" "SnapToTarget" "SnapToTarget" true)
      (`self.K2_AddActorLocalOffset` _returnvalue (0.0 0.0 120.0) false false)
      (set `Actor.CustomTimeDilation` 4.0 _returnvalue)
      (set `self.SmokeActorRef` _returnvalue))
    (:`then_2`
      (return))))

(fn `UserConstructionScript`)