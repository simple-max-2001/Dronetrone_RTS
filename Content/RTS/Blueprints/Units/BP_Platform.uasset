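; BP_Platform is an RTS unit actor that plays destruction effects when its EntityComponent reports death.
; An optional DieOnStartUp flag kills the entity on BeginPlay.
; On death it prints a debug message and calls DeathFX, which spawns an explosion above the platform.
; DeathFX also attaches a raised smoke actor to the platform with its time dilation sped up.
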(event `self.ReceiveBeginPlay`
  (if (`self.bDieOnStartUp`)
    (`EntityComponent.KillEntity` (`self.EntityComponent`))))

(event `self.EntityComponent.OnDieEntity`
  (`KismetSystemLibrary.PrintText` (`|FormatText` "OnDieEntity: {Name}" (`KismetSystemLibrary.GetDisplayName` self)))
  (`self.DeathFX`))

(fn `DeathFX`
  (bind (_returnvalue_location _returnvalue_rotation _returnvalue_scale) (`KismetMathLibrary.BreakTransform` (`self.GetTransform`)))
  (`|ExecutionSequence`
    (:`then_0`
      ;[1 1 1] Add explosion
      (`|SpawnActorFromClass` "/Game/RTS/Blueprints/FX/BP_Explosion.BP_Explosion_C" (`KismetMathLibrary.MakeTransform` (+ _returnvalue_location (0.0 0.0 100.0)) _returnvalue_rotation _returnvalue_scale) "AlwaysSpawn" "MultiplyWithRoot" null null))
    (:`then_1`
      ;[1 1 1] Add smoke
      (bind _returnvalue (`|SpawnActorFromClass` "/Game/RTS/Blueprints/FX/BP_Smoke.BP_Smoke_C" (`self.GetTransform`) "AlwaysSpawn" "MultiplyWithRoot" self null))
      (`self.K2_AttachToActor` _returnvalue self "None" "SnapToTarget" "SnapToTarget" "SnapToTarget" true)
      (`self.K2_AddActorLocalOffset` _returnvalue (0.0 0.0 120.0) false false)
      (set `Actor.CustomTimeDilation` 4.0 _returnvalue))
    (:`then_2`
      (return))))

(fn `UserConstructionScript`)