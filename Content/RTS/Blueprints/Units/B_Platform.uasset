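; RTS platform unit that logs its spawn, death and destroy lifecycle from EntityComponent events.
; When the Die flag is set, BeginPlay starts a looping timer, apparently for the DieOnStartup debug damage through HealthComponent.
; Death spawns an explosion and attached, time-dilated smoke, then a delayed timer calls DestroyEntity on EntityComponent.
; The destroy event also removes the smoke actor.
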(event `self.ReceiveBeginPlay`
  (`self.HealthComponent`
    (:`then`
      (`self.EntityComponent`
        (:`then`
          (if (`self.bDie`)
            (`KismetSystemLibrary.K2_SetTimerDelegate` (`|CreateDelegate` :!event `DieOnStartup`) 1.0 true)))
        (:`else`
          (`KismetSystemLibrary.PrintString` "EntityNotValid" true true (struct :`R` 1.0 :`A` 1.0)))))
    (:`else`
      (`KismetSystemLibrary.PrintString` "HealthNotValid" true true (struct :`R` 1.0 :`A` 1.0)))))

(event `DieOnStartup`
  (bind _healthcomponent (`self.HealthComponent`))
  (bind _healthcomponent_2 (`self.HealthComponent`))
  (`KismetSystemLibrary.PrintText` (`|FormatText` "HealthBefore: {hp} ({hp_p}%) Alive: {alive}" (`HealthComponent.GetHealth` _healthcomponent) (* (`HealthComponent.GetHealthPercentage` _healthcomponent) 100.0) (`EntityComponent.bIsAlive` (`self.EntityComponent`))))
  (`HealthComponent.TakeDamage` (`self.HealthComponent`) (make `DamageData` 20.0))
  (`KismetSystemLibrary.PrintText` (`|FormatText` "HealthAfter: {hp} ({hp_p}%) Alive: {alive}" (`HealthComponent.GetHealth` _healthcomponent_2) (* (`HealthComponent.GetHealthPercentage` _healthcomponent_2) 100.0) (`EntityComponent.bIsAlive` (`self.EntityComponent`)))))

(event `self.EntityComponent.OnSpawnEntity`
  ;[1 1 1] On spawn
  (`KismetSystemLibrary.PrintText` (`|FormatText` "OnSpawnEntity: {Name}" (`KismetSystemLibrary.GetDisplayName` self))))

(event `self.EntityComponent.OnDieEntity`
  ;[1 1 1] On Death
  (`KismetSystemLibrary.PrintText` (`|FormatText` "OnDieEntity: {Name}" (`KismetSystemLibrary.GetDisplayName` self)))
  (`self.DeathFX`)
  (`KismetSystemLibrary.K2_SetTimerDelegate` (delegate `DestroyEvent`) 3.0))

(event `self.EntityComponent.OnDestroyEntity`
  ;[1 1 1] On Destroy
  (`KismetSystemLibrary.PrintText` (`|FormatText` "OnDestroyEntity: {Name}" (`KismetSystemLibrary.GetDisplayName` self)))
  (bind _smokeactorref (`self.SmokeActorRef`)
    (:`then`
      (`self.K2_DestroyActor` _smokeactorref))
    (:`else`)))

(event `DestroyEvent`
  ;[1 1 1] On Death
  (`EntityComponent.DestroyEntity` (`self.EntityComponent`)))

(fn `DeathFX`
  (bind (_returnvalue_location _returnvalue_rotation _returnvalue_scale) (`KismetMathLibrary.BreakTransform` (`self.GetTransform`)))
  (`|ExecutionSequence`
    (:`then_0`
      ;[1 1 1] Add explosion
      (`|SpawnActorFromClass` "/Game/RTS/Blueprints/FX/BP_Explosion.BP_Explosion_C" (`KismetMathLibrary.MakeTransform` (+ _returnvalue_location (0.0 0.0 100.0)) _returnvalue_rotation _returnvalue_scale) "AlwaysSpawn" "MultiplyWithRoot" null null))
    (:`then_1`
      ;[1 1 1] Add smoke
      (bind _returnvalue (`|SpawnActorFromClass` "/Game/RTS/Blueprints/FX/BP_Smoke.BP_Smoke_C" (`self.GetTransform`) "AlwaysSpawn" "MultiplyWithRoot" self null))
      (`self.K2_AttachToActor` _returnvalue self "None" "SnapToTarget" "SnapToTarget" "SnapToTarget" true)
      (`self.K2_AddActorLocalOffset` _returnvalue (0.0 0.0 120.0) false false)
      (set `Actor.CustomTimeDilation` 4.0 _returnvalue)
      (set `self.SmokeActorRef` _returnvalue))
    (:`then_2`
      (return))))

(fn `UserConstructionScript`)